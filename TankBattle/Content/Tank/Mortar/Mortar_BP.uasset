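; Mortar Blueprint that sets up a stationary-or-mobile weapon's aiming and health display when play begins.
; BeginPlay initialises the TankAiming component with TankBarrel as the barrel and Dome as the turret.
; It then casts the Widget component's user widget to HealthBar and hands it a reference to itself as TankHealth.
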(event EventBeginPlay
  (Class|TankAimingComponent|Initialise (Variables|Default|GetTankAiming) (Variables|Default|GetTankBarrel) (Variables|Default|GetDome))
  (CallFunction|InitialiseHealthBar))

(fn ConstructionScript)

(fn InitialiseHealthBar
  (bind _ashealth_bar (Utilities|Casting|CastToHealthBar (UserInterface|GetUserWidgetObject (Variables|Default|GetWidget))))
  (Variables|/Game/UI/HealthBar.HealthBar_C|SetTankHealth _ashealth_bar self)
  (return))